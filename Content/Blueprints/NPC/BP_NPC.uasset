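; Base NPC Blueprint that seeds its AI and manages hand-prop accessories and an auxiliary collision component.
; On possession, it writes its movement direction to the TargetDirection Blackboard key.
; Gameplay-tag switches show or hide the cellphone and cigarette, and the cigarette can be re-attached to a given mesh bone.
; A separate event toggles the PlayerCollisionWhenInvisible component between query-and-physics and no collision.
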(event Custom|ShowAccessory
  (params (Tag :type Gameplay%20Tag%20Structure))
  (|SwitchGameplayTag Tag
    (:Accessory.Cellphone
      (Development|SetHiddeninGame (Variables|Default|GetCellPhone) false false))
    (:Accessory.Cigarette
      (Development|SetHiddeninGame (Variables|Default|GetCigarette) false false))))

(event Custom|HideAccessory
  (params (Tag :type Gameplay%20Tag%20Structure))
  (|SwitchGameplayTag Tag
    (:Accessory.Cellphone
      (Development|SetHiddeninGame (Variables|Default|GetCellPhone) true false))
    (:Accessory.Cigarette
      (Development|SetHiddeninGame (Variables|Default|GetCigarette) true false))))

(event Custom|AttachCigarette
  (params (BoneName :type Name))
  (Transformation|AttachComponentToComponent (Variables|Default|GetCigarette) (Variables|Character|GetMesh) BoneName "SnapToTarget" "SnapToTarget" "KeepRelative" true))

(event Custom|ToggleWhenInvisibleCollision
  (params (IsEnabled :type Boolean))
  (Collision|SetCollisionEnabled (Variables|Default|GetPlayerCollision_WhenInvisible) (select IsEnabled "QueryAndPhysics" "NoCollision")))

(event EventPossessed
  (params (NewController :type Controller%20Object%20Reference))
  (AI|Components|Blackboard|SetValueasVector (AI|GetBlackboard 0) (Utilities|Name|MakeLiteralName "TargetDirection") (Variables|Default|GetMovementDirection)))

(fn ConstructionScript)